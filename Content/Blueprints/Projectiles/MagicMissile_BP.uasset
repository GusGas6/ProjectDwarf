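; Magic missile projectile Blueprint that resolves its first hit with an effect, damage and a physics push.
; A DoOnce-guarded Hit event spawns a spellcast emitter, applies point damage and adds a constant-falloff radial velocity impulse to the struck component.
; It also spawns Alert_AoE_BP at the impact point, then disables Sphere collision and destroys itself after a short delay.
; The damage direction runs from the actor's location to itself, so it is zero.
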(event Collision|EventHit
  (params (MyComp :type Primitive%20Component%20Object%20Reference) (Other :type Actor%20Object%20Reference) (OtherComp :type Primitive%20Component%20Object%20Reference) (bSelfMoved :type Boolean) (HitLocation :type Vector :default "0, 0, 0") (HitNormal :type Vector :default "0, 0, 0") (NormalImpulse :type Vector :default "0, 0, 0") (Hit :type Hit%20Result%20Structure%20%28by%20ref%29))
  (Utilities|FlowControl|DoOnce false
    (:Completed
      (Effects|SpawnEmitteratLocation "/Game/VFX/P_OrbSpellcast.P_OrbSpellcast" HitLocation "0, 0, 0" "0.500000,0.500000,0.500000")
      (Game|Damage|ApplyPointDamage Other 1.0 (Math|Vector|GetUnitDirection(Vector) (Transformation|GetActorLocation) (Transformation|GetActorLocation)) Hit 0 self)
      (Physics|AddRadialImpulse OtherComp (Transformation|GetActorLocation) 4e+03 4e+03 "RIF_Constant" true)
      (Game|SpawnActorfromClass "/Game/Blueprints/AI/Alert_AoE_BP.Alert_AoE_BP_C" (Math|Transform|MakeTransform HitLocation "0, 0, 0" "1.000000,1.000000,1.000000") "Undefined" "MultiplyWithRoot" 0 5e+02 0)
      (Collision|SetCollisionEnabled (Variables|Default|GetSphere) "NoCollision")
      (Utilities|FlowControl|Delay 0.5)
      (Actor|DestroyActor))))

(fn ConstructionScript)