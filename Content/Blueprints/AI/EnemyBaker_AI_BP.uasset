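; EnemyBaker AI is a dormant enemy that wakes when a third-person character enters its radius, then chases players.
; The overlap fires once, sets Attacking, starts both loops and destroys the wake-up sphere through SERVER- and CLIENT-named events.
; A chase loop reissues AIMoveTo to the target player's current location each tick.
; A self-calling delay loop alternates the target between player indices 0 and 1 every two seconds, regardless of distance.
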(event OnComponentBeginOverlap(WakeUpRadius)
  (params (OverlappedComponent :type Primitive%20Component%20Object%20Reference) (OtherActor :type Actor%20Object%20Reference) (OtherComp :type Primitive%20Component%20Object%20Reference) (OtherBodyIndex :type Integer) (bFromSweep :type Boolean) (SweepResult :type Hit%20Result%20Structure%20%28by%20ref%29))
  (Utilities|Casting|CastToBP_ThirdPersonCharacter OtherActor)
  (Utilities|FlowControl|DoOnce false
    (:Completed
      (CallFunction|SERVERChasePlayer))))

(event Custom|CLIENT%20Remove%20Collision%20Sphere
  (Components|DestroyComponent (Variables|Default|GetWakeUpRadius)))

(event Custom|ChaseLoop
  (AI|AIMoveTo self (Transformation|GetActorLocation (Game|GetPlayerCharacter (Variables|Default|GetPlayer%20Index))) 0 5.0 false
    (:then
      (Utilities|FlowControl|DelayUntilNextTick)
      (CallFunction|ChaseLoop))))

(event Custom|SwapTarget
  (params (Delay :type Float%20%28double-precision%29))
  (Utilities|FlowControl|Delay Delay)
  (if (== (Variables|Default|GetPlayer%20Index) 0)
    (Variables|Default|SetPlayer%20Index 1)
    (else
      (Variables|Default|SetPlayer%20Index 0)))
  (CallFunction|SwapTarget 2.0))

(event Custom|SERVER%20ChasePlayer
  (Variables|Default|SetAttacking true)
  (CallFunction|ChaseLoop)
  (CallFunction|SwapTarget 2.0)
  (CallFunction|CLIENTRemoveCollisionSphere))

(fn ConstructionScript)