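; Game instance that handles online friend sessions through Advanced Sessions, covering session creation and invite-based joining.
; CreateSession makes a session and, after a short delay, opens the waiting-for-players map as a listen server.
; Accepting an invite joins the session, then calls PlayerFound on waiting-screen widgets in that same instance and triggers LoadLevelOnJoin.
; LoadLevelOnJoin runs once, calling a delayed ServerTravel to TransitionMap from the joining side and printing the result.
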(event Custom|CreateSession
  ;[1 1 1] Create Session
  (|AdvancedSession 0 (Game|GetPlayerController 0) 100 0 false true false true true true false false false true false true
    (:OnSuccess
      (Utilities|FlowControl|Delay 3.0)
      (Game|OpenLevel(byObjectReference) "/Game/Maps/MainMenuMap_WaitingForPlayers.MainMenuMap_WaitingForPlayers" true "listen"))))

(event Custom|LoadLevelOnJoin
  ;[1 1 1] Load Level On Join
  (Utilities|FlowControl|DoOnce false
    (:Completed
      (Utilities|FlowControl|Delay 3.0)
      (bind _returnvalue (Class|AdvancedSessionsLibrary|ServerTravel "TransitionMap" false false))
      (Development|PrintString (Utilities|String|ToString(Boolean) _returnvalue)))))

(event EventOnSessionInviteAccepted
  (params (LocalPlayerNum :type Integer) (PersonInvited :type BP%20Unique%20Net%20Id%20Structure) (SessionToJoin :type Blueprint%20Session%20Result%20Structure%20%28by%20ref%29))
  ;[1 1 1] Join Session (via invite)
  (|JoinSession (Game|GetPlayerController 0) SessionToJoin
    (:OnSuccess
      (Utilities|FlowControl|Sequence
        (:then_0
          (bind _foundwidgets (Widget|GetAllWidgetsOfClass "/Game/UI/WaitingForPlayersOnline_WBP.WaitingForPlayersOnline_WBP_C" true))
          (for _array_element _foundwidgets
            (Utilities|IsValid _array_element
              (:Is%20Valid
                (Default|PlayerFound _array_element)))))
        (:then_1
          (CallFunction|LoadLevelonJoin))))))